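; Demo player character with movement, look and inventory-opening input for a Jigsaw inventory component.
; BeginPlay registers the default Enhanced Input mapping context and adds the HUD widget to the viewport.
; Move input follows the control rotation's yaw, and look input drives controller yaw and pitch.
; The open-inventory action calls the component's opened and updated notifications in turn.
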(event `self.ReceiveBeginPlay`
  (bind _asplayer_controller (cast `PlayerController` (`self.GetController`)))
  (`EnhancedInputSubsystemInterface.AddMappingContext` (pcsubsystem `EnhancedInputLocalPlayerSubsystem` _asplayer_controller) "/CompleteJigsawInventory/Input/IMC_Default.IMC_Default" 0 (struct))
  (bind _returnvalue (`|CreateWidget` "/CompleteJigsawInventory/Widgets/WBP_HUD.WBP_HUD_C" _asplayer_controller))
  (`UserWidget.AddToViewport` _returnvalue 0))

(event `Key|Tab`
  (params (Key :type "Key Structure")))

(event `EnhancedInput|/CompleteJigsawInventory/Input/IA_OpenInventory`
  (params (ActionValue :type Boolean) (ElapsedSeconds :type "Float (double-precision)") (TriggeredSeconds :type "Float (double-precision)") (InputAction :type "InputAction Object Reference" :default "/CompleteJigsawInventory/Input/IA_OpenInventory.IA_OpenInventory"))
  (bind _jigsawinventory (`self.JigsawInventory`))
  (:`Triggered`
    (`JigsawInventoryComponent.OnInventoryOpened` _jigsawinventory)
    (`JigsawInventoryComponent.OnInventoryUpdated` _jigsawinventory)))

(event `EnhancedInput|/CompleteJigsawInventory/Input/IA_SplitItem`
  (params (ActionValue :type Boolean) (ElapsedSeconds :type "Float (double-precision)") (TriggeredSeconds :type "Float (double-precision)") (InputAction :type "InputAction Object Reference" :default "/CompleteJigsawInventory/Input/IA_SplitItem.IA_SplitItem")))

(event `EnhancedInput|/CompleteJigsawInventory/Input/IA_HalveStack`
  (params (ActionValue :type Boolean) (ElapsedSeconds :type "Float (double-precision)") (TriggeredSeconds :type "Float (double-precision)") (InputAction :type "InputAction Object Reference" :default "/CompleteJigsawInventory/Input/IA_HalveStack.IA_HalveStack")))

(event `EnhancedInput|/CompleteJigsawInventory/Input/Default/IA_Move`
  (params (ActionValue :type "Vector2D Structure") (ElapsedSeconds :type "Float (double-precision)") (TriggeredSeconds :type "Float (double-precision)") (InputAction :type "InputAction Object Reference" :default "/CompleteJigsawInventory/Input/Default/IA_Move.IA_Move"))
  (bind (_returnvalue_roll _returnvalue_pitch _returnvalue_yaw) (`KismetMathLibrary.BreakRotator` (`self.GetControlRotation`)))
  (bind (_x _y) (`KismetMathLibrary.BreakVector2D` ActionValue))
  (bind (_x_2 _y_2) (`KismetMathLibrary.GetAxes` (`KismetMathLibrary.MakeRotator` 0.0 0.0 _returnvalue_yaw)))
  ;[0 0 0] Default Movement Controls
  (:`Triggered`
    (`self.AddMovementInput` _x_2 _y)
    (`self.AddMovementInput` _y_2 _x)))

(event `EnhancedInput|/CompleteJigsawInventory/Input/Default/IA_Look`
  (params (ActionValue :type "Vector2D Structure") (ElapsedSeconds :type "Float (double-precision)") (TriggeredSeconds :type "Float (double-precision)") (InputAction :type "InputAction Object Reference" :default "/CompleteJigsawInventory/Input/Default/IA_Look.IA_Look"))
  (bind (_x _y) (`KismetMathLibrary.BreakVector2D` ActionValue))
  ;[0 0 0] Default Movement Controls
  (:`Triggered`
    (`self.AddControllerYawInput` _x)
    (`self.AddControllerPitchInput` _y)))

(fn `UserConstructionScript`)